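; BP_Button is a one-shot button in the gravity objects set that triggers a linked trap door.
; Activating works only while CanBeActivated is true, then clears it and plays a Timeline scaled to last TimeClose, assuming a one-second track.
; The Timeline lerps the Sphere's relative Z to a fixed height.
; On finish, the sphere turns unlit green and calls OpenAndSpawn on TrapDoorRef if valid.
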(event EventActivating
  (params (Player :type BP%20First%20Person%20Character%20Object%20Reference))
  (bind _sphere (Variables|Default|GetSphere))
  (bind _trapdoor_ref (Variables|Default|GetTrapDoor_ref))
  (bind _relativelocation (Variables|/Script/Engine.SceneComponent|GetRelativeLocation _sphere))
  (if (Variables|Default|GetCanBeActivated?)
    (Variables|Default|SetCanBeActivated? false)
    (Components|Timeline|SetPlayRate (Variables|Default|GetTimeline) (/ 1.0 (Variables|Default|GetTimeClose)))
    (Variables|Default|SetSphereLoc_OG (.z _relativelocation))
    (bind _newtrack_0 (Timeline|Timeline PlayFromStart)
      (:Update
        (Transformation|SetRelativeLocation (Variables|Default|GetSphere) (Math|Vector|MakeVector (.x _relativelocation) (.y _relativelocation) (Math|Float|Lerp (Variables|Default|GetSphereLoc_OG) 87.0 _newtrack_0)) false false))
      (:Finished
        (Rendering|Material|SetMaterial (Variables|Default|GetSphere) 0 "/Game/StarterBundle/ModularScifiProps/Materials/MI_Light_Green_Unlit.MI_Light_Green_Unlit")
        (Utilities|IsValid _trapdoor_ref
          (:Is%20Valid
            (Default|OpenandSpawn _trapdoor_ref)))))))

(fn ConstructionScript)