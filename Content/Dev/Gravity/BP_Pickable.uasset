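; BP_Pickable is an interactable object that the player can pick up, with an outline overlay while it is seen.
; On activation, if pickable, it halves its mesh scale, limits blocking to world static and one custom channel, zeroes its mass override and calls the player's Grab.
; ReScale restores original scale, broad collision and a heavy mass, and zeroes rotation for BP_GravityForce_Current instances.
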(event EventBeginPlay
  (Variables|Default|SetOGScale (Transformation|GetWorldScale (Variables|Default|GetStaticMesh))))

(event EventIsSeen
  (params (isSeen :type Boolean))
  (Rendering|Material|SetOverlayMaterial (Variables|Default|GetStaticMesh) (select isSeen "/Game/Dev/Materials/M_Outline.M_Outline" 0) :!class /Script/Engine.MeshComponent))

(event EventActivating
  (params (Player :type BP%20First%20Person%20Character%20Object%20Reference))
  (bind _staticmesh (Variables|Default|GetStaticMesh))
  (if (Variables|Default|GetCanBePicked)
    (Transformation|SetWorldScale3D _staticmesh (* (Variables|Default|GetOGScale) "0.500000,0.500000,0.500000"))
    (Collision|SetCollisionResponsetoAllChannels _staticmesh "ECR_Ignore")
    (Collision|SetCollisionResponsetoChannel _staticmesh "ECC_GameTraceChannel3" "ECR_Block")
    (Collision|SetCollisionResponsetoChannel _staticmesh "ECC_WorldStatic" "ECR_Block")
    (Class|PrimitiveComponent|SetMassOverrideinKg (Variables|Default|GetStaticMesh) "None" 0.0 true)
    (Default|Grab Player self)))

(fn ConstructionScript)

(fn ReScale
  (bind _self self)
  (bind _staticmesh (Variables|Default|GetStaticMesh))
  (Transformation|SetWorldScale3D _staticmesh (Variables|Default|GetOGScale))
  (Collision|SetCollisionResponsetoAllChannels _staticmesh "ECR_Block")
  (Collision|SetCollisionResponsetoChannel _staticmesh "ECC_GameTraceChannel4" "ECR_Ignore")
  (Class|PrimitiveComponent|SetMassOverrideinKg (Variables|Default|GetStaticMesh) "None" 1e+03 true)
  (Utilities|Casting|CastToBP_GravityForce_Current _self)
  (Transformation|SetActorRotation _self))