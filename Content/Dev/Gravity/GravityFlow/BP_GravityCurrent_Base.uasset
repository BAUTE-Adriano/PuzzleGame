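; Base gravity current actor: a box volume that, while activated, affects any BP_GravityObject that begins overlapping it.
; BeginPlay sizes the box from BasePerimeter and Height.
; On overlap, it switches off physics simulation on the object's Cube and calls GravityInverted with the current's up vector scaled by the box's Z extent.
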(event OnComponentBeginOverlap(Box)
  (params (OverlappedComponent :type Primitive%20Component%20Object%20Reference) (OtherActor :type Actor%20Object%20Reference) (OtherComp :type Primitive%20Component%20Object%20Reference) (OtherBodyIndex :type Integer) (bFromSweep :type Boolean) (SweepResult :type Hit%20Result%20Structure%20%28by%20ref%29))
  (if (Variables|Status|GetisActivated)
    (bind _asbp_gravity_activeable_base (Utilities|Casting|CastToBP_GravityObject OtherActor))
    (CallFunction|GravityParametersSetUp _asbp_gravity_activeable_base)))

(event EventBeginPlay
  (CallFunction|SetBoxSize))

(fn ConstructionScript)

(fn SetBoxSize
  (bind _baseperimeter (Variables|FlowParameters|GetBasePerimeter))
  (Components|Box|SetBoxExtent (Variables|Default|GetBox) (Math|Vector|MakeVector _baseperimeter _baseperimeter (Variables|FlowParameters|GetHeight)) true)
  (return))

(fn GravityParametersSetUp
  (params (Actor :type BP%20Gravity%20Object%20Object%20Reference))
  (Physics|SetSimulatePhysics (Variables|/Game/Dev/Gravity/GravityObjects/BP_GravityObject.BP_GravityObject_C|GetCube Actor) (not (Variables|Status|GetisActivated)))
  (Default|GravityInverted Actor (CallFunction|GetDirection))
  (return))

(fn GetDirection
  (return (* (Transformation|GetActorUpVector) (.z (Variables|/Script/Engine.BoxComponent|GetBoxExtent (Variables|Default|GetBox))))))