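; BP_GravityForce_Current is a box volume that pushes a BP_GravityObject along its Direction forward vector, like a current.
; On overlap it disables the object's gravity, clears every other current's object reference and starts a looping timer.
; The timer calls Attract, which applies CurrentStrength as force while IsActivated.
; On exit it clears its reference and timer, restoring gravity if no other current overlaps the object.
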(event OnComponentBeginOverlap(Box)
  (params (OverlappedComponent :type Primitive%20Component%20Object%20Reference) (OtherActor :type Actor%20Object%20Reference) (OtherComp :type Primitive%20Component%20Object%20Reference) (OtherBodyIndex :type Integer) (bFromSweep :type Boolean) (SweepResult :type Hit%20Result%20Structure%20%28by%20ref%29))
  (bind _asbp_gravity_object (Utilities|Casting|CastToBP_GravityObject OtherActor))
  (bind _output_get (Variables|Default|SetAs%20BP%20Gravity%20Object _asbp_gravity_object))
  (Default|ActivateDeactivateGravity _output_get false)
  (bind _returnvalue (Utilities|Time|SetTimerbyFunctionName 0 "Attract" 0.3 true))
  (Variables|Default|SetAttractTimer_Handle _returnvalue)
  (bind _outactors (Actor|GetAllActorsOfClass "BP_GravityForce_Current_C"))
  (for _array_element _outactors
    (if (!= _array_element self)
      (Variables|BP_GravityForce_Current_C|SetAs%20BP%20Gravity%20Object _array_element 0))))

(event OnComponentEndOverlap(Box)
  (params (OverlappedComponent :type Primitive%20Component%20Object%20Reference) (OtherActor :type Actor%20Object%20Reference) (OtherComp :type Primitive%20Component%20Object%20Reference) (OtherBodyIndex :type Integer))
  (bind _asbp_gravity_object (Utilities|Casting|CastToBP_GravityObject OtherActor))
  (Utilities|FlowControl|Sequence
    (:then_0
      (if (Utilities|Array|IsEmpty (Collision|GetOverlappingActors (Variables|/Game/Dev/Gravity/BP_PickUpObject.BP_PickUpObject_C|GetCube _asbp_gravity_object) "BP_GravityForce_Current_C" :!class /Script/Engine.PrimitiveComponent))
        (Default|ActivateDeactivateGravity _asbp_gravity_object true)
        (else
          (Development|PrintString "Hello"))))
    (:then_1
      (Variables|Default|SetAs%20BP%20Gravity%20Object 0)
      (Utilities|Time|ClearandInvalidateTimerbyHandle (Variables|Default|GetAttractTimer_Handle)))))

(event EventTick
  (params (DeltaSeconds :type Float%20%28single-precision%29)))

(fn ConstructionScript)

(fn Attract
  (if (and (Variables|Default|GetisActivated) (Utilities|IsValid (Variables|Default|GetAs%20BP%20Gravity%20Object)))
    (Physics|AddForce (Variables|/Game/Dev/Gravity/BP_PickUpObject.BP_PickUpObject_C|GetCube (Variables|Default|GetAs%20BP%20Gravity%20Object)) (* (Math|Vector|GetForwardVector (Variables|Default|GetDirection)) (Variables|Default|GetCurrentStrength)) "None" false)))