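; BP_GravityCurrent is a box volume that carries an overlapping BP_GravityObject along the actor's up vector.
; On overlap it disables the cube's physics, and the Elevation timeline offsets it from its entry point by up to the box's Z extent over TimeOfMovement, printing each position.
; Leaving the box stops the timeline and restores physics for the single tracked object.
; BeginPlay bakes the box's scale into its extent.
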(event OnComponentBeginOverlap(Box)
  (params (OverlappedComponent :type Primitive%20Component%20Object%20Reference) (OtherActor :type Actor%20Object%20Reference) (OtherComp :type Primitive%20Component%20Object%20Reference) (OtherBodyIndex :type Integer) (bFromSweep :type Boolean) (SweepResult :type Hit%20Result%20Structure%20%28by%20ref%29))
  (bind _asbp_gravity_object (Utilities|Casting|CastToBP_GravityObject OtherActor))
  (bind _output_get (Variables|Default|SetGravityObject_ref _asbp_gravity_object))
  (Physics|SetSimulatePhysics (Variables|/Game/Dev/Gravity/BP_PickUpObject.BP_PickUpObject_C|GetCube _output_get) false)
  (Variables|Default|SetInitialLocation (Transformation|GetWorldLocation (Variables|/Game/Dev/Gravity/BP_PickUpObject.BP_PickUpObject_C|GetCube _output_get)))
  (Components|Timeline|SetPlayRate (Variables|Default|GetElevation) (/ 1.0 (Variables|Default|GetTimeOfMovement)))
  (bind _normalized_position (Timeline|Elevation Play)
    (:Update
      (Transformation|SetWorldLocation (Variables|/Game/Dev/Gravity/BP_PickUpObject.BP_PickUpObject_C|GetCube (Variables|Default|GetGravityObject_ref)) (+ (Variables|Default|GetInitialLocation) (* _normalized_position (* (Transformation|GetActorUpVector) (.z (Components|Box|GetScaledBoxExtent (Variables|Default|GetBox)))))) false false)
      (Development|PrintString (Utilities|String|ToString(Vector) (+ (Variables|Default|GetInitialLocation) (* _normalized_position (* (Transformation|GetActorUpVector) (.z (Components|Box|GetScaledBoxExtent (Variables|Default|GetBox)))))))))))

(event OnComponentEndOverlap(Box)
  (params (OverlappedComponent :type Primitive%20Component%20Object%20Reference) (OtherActor :type Actor%20Object%20Reference) (OtherComp :type Primitive%20Component%20Object%20Reference) (OtherBodyIndex :type Integer))
  (if (== (Variables|Default|GetGravityObject_ref) OtherActor)
    (Audio|Components|Audio|Stop (Variables|Default|GetElevation))
    (Physics|SetSimulatePhysics (Variables|/Game/Dev/Gravity/BP_PickUpObject.BP_PickUpObject_C|GetCube (Variables|Default|GetGravityObject_ref)) true)
    (Variables|Default|SetGravityObject_ref 0)))

(event EventBeginPlay
  (bind _box (Variables|Default|GetBox))
  (Components|Box|SetBoxExtent _box (Components|Box|GetScaledBoxExtent _box) true)
  (Transformation|SetWorldScale3D _box "1.000000,1.000000,1.000000"))

(fn ConstructionScript)