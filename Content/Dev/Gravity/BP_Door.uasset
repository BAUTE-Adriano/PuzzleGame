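; BP_Door is a level-exit door in the Gravity dev folder that checks whether every BP_PushOn actor is activated.
; On BeginPlay it gathers all BP_PushOn actors and binds an open check to their HasBeenActivated event.
; The check loops over their Activated flags, stops at the first inactive one, and calls FinishLevel when all are active.
; FinishLevel is currently an empty stub.
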(event Custom|Open?
  (bind _array_element (Utilities|Array|ForEachLoopwithBreak (stale EventBeginPlay _outactors) :!label _label)
    (:LoopBody
      (if (Variables|/Game/Dev/Gravity/BP_PushOn.BP_PushOn_C|GetActivated _array_element)
        (Variables|Default|SetAllActivated true)
        (else
          (Variables|Default|SetAllActivated false)
          (goto _label Break))))
    (:Completed
      (if (Variables|Default|GetAllActivated)
        (CallFunction|FinishLevel)))))

(event EventBeginPlay
  (bind _outactors (Actor|GetAllActorsOfClass "/Game/Dev/Gravity/BP_PushOn.BP_PushOn_C"))
  (EventDispatchers|BindEventtoHasBeenActivated _outactors (delegate Custom|Open?)))

(fn ConstructionScript)

(fn FinishLevel)