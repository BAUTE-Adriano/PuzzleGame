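; Pressure plate switch that activates when an actor implementing I_Weight overlaps its Box and deactivates when one leaves.
; Separate press and release timelines, rate-scaled by Speed, move the mesh vertically and swap its trim between orange and red.
; Activation also toggles an outline overlay, and both timelines fire CallHasBeenActivated on every update.
; The IsSeen event checks the player's grabbed object but takes no action.
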(event OnComponentBeginOverlap(Box)
  (params (OverlappedComponent :type Primitive%20Component%20Object%20Reference) (OtherActor :type Actor%20Object%20Reference) (OtherComp :type Primitive%20Component%20Object%20Reference) (OtherBodyIndex :type Integer) (bFromSweep :type Boolean) (SweepResult :type Hit%20Result%20Structure%20%28by%20ref%29))
  (bind _staticmesh (Variables|Default|GetStaticMesh))
  (if (Utilities|DoesObjectImplementInterface OtherActor "/Game/Dev/Gravity/I_Weight.I_Weight_C")
    (Variables|Default|SetActivated true)
    (Rendering|Material|SetOverlayMaterial (Variables|Default|GetPressPlate) "/Game/Dev/Materials/M_ActivatedOutline.M_ActivatedOutline" :!class /Script/Engine.MeshComponent)
    (Components|Timeline|SetPlayRate (Variables|Default|GetPress) (/ 1.0 (Variables|Default|GetSpeed)))
    (bind _newtrack_0 (Timeline|Press Play)
      (:Update
        (Transformation|SetRelativeLocation (Variables|Default|GetStaticMesh) (Math|Vector|MakeVector 0.0 0.0 (Math|Float|Lerp 8.0 5.5 _newtrack_0)) false false)
        (Rendering|Material|SetMaterial _staticmesh 0 "/Game/StarterBundle/ModularSci_Comm/Materials/MI_Trims_C_Orange.MI_Trims_C_Orange")
        (Rendering|Material|SetMaterial _staticmesh 3 "/Game/StarterBundle/ModularSci_Comm/Materials/MI_Trims_C_Orange.MI_Trims_C_Orange")
        (Default|CallHasBeenActivated)))))

(event OnComponentEndOverlap(Box)
  (params (OverlappedComponent :type Primitive%20Component%20Object%20Reference) (OtherActor :type Actor%20Object%20Reference) (OtherComp :type Primitive%20Component%20Object%20Reference) (OtherBodyIndex :type Integer))
  (bind _staticmesh (Variables|Default|GetStaticMesh))
  (if (Utilities|DoesObjectImplementInterface OtherActor "/Game/Dev/Gravity/I_Weight.I_Weight_C")
    (Variables|Default|SetActivated false)
    (Rendering|Material|SetOverlayMaterial (Variables|Default|GetPressPlate) 0 :!class /Script/Engine.MeshComponent)
    (Components|Timeline|SetPlayRate (Variables|Default|GetTimeline) (Variables|Default|GetSpeed))
    (bind _newtrack_0 (Timeline|Timeline Reverse)
      (:Update
        (Transformation|SetRelativeLocation (Variables|Default|GetStaticMesh) (Math|Vector|MakeVector 0.0 0.0 (Math|Float|Lerp 8.0 5.5 _newtrack_0)) false false)
        (Rendering|Material|SetMaterial _staticmesh 0 "/Game/StarterBundle/ModularSci_Comm/Materials/MI_Trims_C_Red.MI_Trims_C_Red")
        (Rendering|Material|SetMaterial _staticmesh 3 "/Game/StarterBundle/ModularSci_Comm/Materials/MI_Trims_C_Red.MI_Trims_C_Red")
        (Default|CallHasBeenActivated)))))

(event EventIsSeen
  (params (isSeen :type Boolean))
  (Utilities|IsValid (Variables|/Game/FirstPerson/Blueprints/BP_FirstPersonCharacter.BP_FirstPersonCharacter_C|GetGrabbedObject (.AsBP%20First%20Person%20Character (Utilities|Casting|CastToBP_FirstPersonCharacter (Game|Player|GetPlayerPawn 0))))))

(fn ConstructionScript)