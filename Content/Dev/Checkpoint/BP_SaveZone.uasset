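; BP_SaveZone is a checkpoint trigger between streamed levels that saves progress when the first-person character enters its box.
; On overlap it starts streaming in the current level and saves that level and the character's HasRemote flag through GI_Main.
; It closes one door with a camera shake, waits briefly, then opens the other and unloads the specified level, working like an airlock that covers the streaming.
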(event OnComponentBeginOverlap(Box)
  (params (OverlappedComponent :type Primitive%20Component%20Object%20Reference) (OtherActor :type Actor%20Object%20Reference) (OtherComp :type Primitive%20Component%20Object%20Reference) (OtherBodyIndex :type Integer) (bFromSweep :type Boolean) (SweepResult :type Hit%20Result%20Structure%20%28by%20ref%29))
  (bind _asbp_first_person_character (Utilities|Casting|CastToBP_FirstPersonCharacter OtherActor))
  (Class|GameplayStatics|LoadStreamLevelbySoftObjectPtr (Variables|Default|GetCurrentLevel) true false)
  (Default|Save (.AsGI%20Main (Utilities|Casting|CastToGI_Main (Game|GetGameInstance))) (Utilities|Struct|MakeSoftWorldReference (Variables|Default|GetCurrentLevel)) (Variables|/Game/FirstPerson/Blueprints/BP_FirstPersonCharacter.BP_FirstPersonCharacter_C|GetHasRemote _asbp_first_person_character))
  (Default|CloseDoor (Variables|Default|GetOpeningDoor))
  (Camera|PlayWorldCameraShake "/Game/Dev/Camera/MovCam_Main.MovCam_Main_C" (Transformation|GetActorLocation) 1e+02 1e+03)
  (Development|PrintString "Hello")
  (Utilities|FlowControl|Delay 3.0)
  (Default|OpenDoors (Variables|Default|GetClosingDoors))
  (Class|GameplayStatics|UnloadStreamLevelbySoftObjectPtr (Variables|Default|GetLevelToUnload) false))

(event EventBeginPlay)

(fn ConstructionScript)