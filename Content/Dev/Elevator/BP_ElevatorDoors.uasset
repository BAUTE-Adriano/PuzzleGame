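; BP_ElevatorDoors is a pair of sliding elevator door panels, built from two wall meshes, with OpenDoors and CloseDoor events.
; OpenDoors caches both panels' relative locations, then a timeline lerps them 100 units apart in opposite directions along local X.
; CloseDoor reverses the same timeline.
; OpenDoors sits behind a DoOnce with no reset in the graph, so it only takes effect once.
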(event Custom|Open%20Doors
  (Utilities|FlowControl|DoOnce false
    (:Completed
      (Variables|Default|SetRelative%20Location (Variables|/Script/Engine.SceneComponent|GetRelativeLocation (Variables|Default|GetWall_A38_StaticMeshComponent0)))
      (Variables|Default|SetRelative%20Location_0 (Variables|/Script/Engine.SceneComponent|GetRelativeLocation (Variables|Default|GetWall_A37_StaticMeshComponent0)))
      (bind _newtrack_0 (Timeline|Timeline Play)
        (:Update
          (Transformation|SetRelativeLocation (Variables|Default|GetWall_A38_StaticMeshComponent0) (Math|Vector|Lerp(Vector) (Variables|Default|GetRelative%20Location) (+ (Variables|Default|GetRelative%20Location) "-100.000000,0.000000,0.000000") _newtrack_0) false false)
          (Transformation|SetRelativeLocation (Variables|Default|GetWall_A37_StaticMeshComponent0) (Math|Vector|Lerp(Vector) (Variables|Default|GetRelative%20Location_0) (+ (Variables|Default|GetRelative%20Location_0) "100.000000,0.000000,0.000000") _newtrack_0) false false))))))

(event Custom|CloseDoor
  (bind _relative_location_0 (Variables|Default|GetRelative%20Location_0))
  (bind _relative_location (Variables|Default|GetRelative%20Location))
  (bind _newtrack_0 (Timeline|Timeline Reverse)
    (:Update
      (Transformation|SetRelativeLocation (Variables|Default|GetWall_A38_StaticMeshComponent0) (Math|Vector|Lerp(Vector) _relative_location (+ _relative_location "-100.000000,0.000000,0.000000") _newtrack_0) false false)
      (Transformation|SetRelativeLocation (Variables|Default|GetWall_A37_StaticMeshComponent0) (Math|Vector|Lerp(Vector) _relative_location_0 (+ _relative_location_0 "100.000000,0.000000,0.000000") _newtrack_0) false false))))

(fn ConstructionScript)