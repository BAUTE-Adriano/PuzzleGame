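; Big sliding door that rises when all linked Plaques are active and reverses at double speed if one deactivates; a first door opens on BeginPlay.
; Spawns a light per plaque above itself, binding each plaque to the check.
; The player's first exit from Box_End blocks pawns, closes the door from its current height, then opens NextDoor.
; A fully opened final door passes level load/unload data to SaveZone and opens its door.
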(event OnComponentEndOverlap(Box_End)
  (params (OverlappedComponent :type Primitive%20Component%20Object%20Reference) (OtherActor :type Actor%20Object%20Reference) (OtherComp :type Primitive%20Component%20Object%20Reference) (OtherBodyIndex :type Integer))
  (bind _sm_door_l_staticmeshcomponent0 (Variables|Default|GetSM_Door_L_StaticMeshComponent0))
  (bind _relativelocation (Variables|/Script/Engine.SceneComponent|GetRelativeLocation _sm_door_l_staticmeshcomponent0))
  ;[0 0.6394 1 0.5] Close Door
  (Utilities|Casting|CastToBP_FirstPersonCharacter OtherActor)
  (Utilities|FlowControl|DoOnce false
    (:Completed
      (Collision|SetCollisionResponsetoChannel (Variables|Default|GetBox) "ECC_Pawn" "ECR_Block")
      (Audio|Components|Audio|Stop (Variables|Default|GetDoor%20Activ))
      (Components|Timeline|SetPlayRate (Variables|Default|GetDoor_Close) (/ 1.0 (Variables|Default|GetTime%20Close)))
      (Variables|Default|SetDoorLocation (.z (Transformation|GetWorldLocation (Variables|Default|GetSM_Door_L_StaticMeshComponent0))))
      (bind _location (Timeline|Door_Close PlayFromStart)
        (:Update
          (Transformation|SetRelativeLocation _sm_door_l_staticmeshcomponent0 (Math|Vector|MakeVector (.x _relativelocation) (.y _relativelocation) (Math|Float|Lerp (Variables|Default|GetDoorLocation) 0.0 _location)) false false))
        (:Finished
          (Variables|Default|SetLocked true)
          (bind _nextdoor (Variables|Default|GetNextDoor)
            (:then
              (CallFunction|NextDoorEvent _nextdoor))
            (:else)))))))

(event Custom|check
  (bind _savezone (Variables|Default|GetSaveZone))
  (bind _sm_door_l_staticmeshcomponent0 (Variables|Default|GetSM_Door_L_StaticMeshComponent0))
  (bind _relativelocation (Variables|/Script/Engine.SceneComponent|GetRelativeLocation _sm_door_l_staticmeshcomponent0))
  ;[0.01176 0.5781 0 0.5] Check Open
  (bind _array_element (Utilities|Array|ForEachLoopwithBreak (Variables|Default|GetPlaques) :!label _label)
    (:LoopBody
      (if (Variables|/Game/Dev/Gravity/BP_PushOn.BP_PushOn_C|GetActivated _array_element)
        (Variables|Default|SetCanBeOpened true)
        (else
          (Variables|Default|SetCanBeOpened false)
          (goto _label Break))))
    (:Completed
      (if (Variables|Default|GetCanBeOpened)
        (Variables|Default|SetLocked false)
        (Components|Timeline|SetPlayRate (Variables|Default|GetDoor%20Activ) (/ 1.0 (Variables|Default|GetTime%20Opening)))
        (bind _location (Timeline|Door%20Activ Play)
          (:Update
            (Transformation|SetRelativeLocation _sm_door_l_staticmeshcomponent0 (Math|Vector|MakeVector (.x _relativelocation) (.y _relativelocation) (Math|Float|Lerp 0.0 3.9e+02 _location)) false false))
          (:Finished
            (if (Variables|Default|GetBFinalDoor)
              (if (Utilities|IsValidSoftObjectReference _savezone)
                (Variables|/Game/Dev/Checkpoint/BP_SaveZone.BP_SaveZone_C|SetCurrentLevel (Utilities|ResolveSoftReference _savezone) (Variables|Default|GetNextLevel))
                (Variables|/Game/Dev/Checkpoint/BP_SaveZone.BP_SaveZone_C|SetLevelToUnload (Utilities|ResolveSoftReference _savezone) (Variables|Default|GetLevelToUnload))
                (Default|OpenDoors (Variables|/Game/Dev/Checkpoint/BP_SaveZone.BP_SaveZone_C|GetOpeningDoor (Utilities|ResolveSoftReference _savezone)))))))
        (else
          (Variables|Default|SetLocked true)
          (Components|Timeline|SetPlayRate (Variables|Default|GetDoor%20Activ) (/ 1.0 (/ (Variables|Default|GetTime%20Opening) 2.0)))
          (Timeline|Door%20Activ Reverse))))))

(event Custom|NextDoorEvent
  (bind _savezone (Variables|Default|GetSaveZone))
  (bind _sm_door_l_staticmeshcomponent0 (Variables|Default|GetSM_Door_L_StaticMeshComponent0))
  (bind _relativelocation (Variables|/Script/Engine.SceneComponent|GetRelativeLocation _sm_door_l_staticmeshcomponent0))
  ;[0.01176 0.5781 0 0.5] Check Open
  (Components|Timeline|SetPlayRate (Variables|Default|GetDoor%20Activ) (/ 1.0 (Variables|Default|GetTime%20Opening)))
  (bind _location (Timeline|Door%20Activ Play)
    (:Update
      (Transformation|SetRelativeLocation _sm_door_l_staticmeshcomponent0 (Math|Vector|MakeVector (.x _relativelocation) (.y _relativelocation) (Math|Float|Lerp 0.0 3.9e+02 _location)) false false))
    (:Finished
      (if (Variables|Default|GetBFinalDoor)
        (if (Utilities|IsValidSoftObjectReference _savezone)
          (Variables|/Game/Dev/Checkpoint/BP_SaveZone.BP_SaveZone_C|SetCurrentLevel (Utilities|ResolveSoftReference _savezone) (Variables|Default|GetNextLevel))
          (Variables|/Game/Dev/Checkpoint/BP_SaveZone.BP_SaveZone_C|SetLevelToUnload (Utilities|ResolveSoftReference _savezone) (Variables|Default|GetLevelToUnload))
          (Default|OpenDoors (Variables|/Game/Dev/Checkpoint/BP_SaveZone.BP_SaveZone_C|GetOpeningDoor (Utilities|ResolveSoftReference _savezone))))))))

(event EventBeginPlay
  (bind _returnvalue (Transformation|GetActorTransform))
  (bind _savezone (Variables|Default|GetSaveZone))
  (bind _sm_door_l_staticmeshcomponent0 (Variables|Default|GetSM_Door_L_StaticMeshComponent0))
  (bind _relativelocation (Variables|/Script/Engine.SceneComponent|GetRelativeLocation _sm_door_l_staticmeshcomponent0))
  ;[0.7812 0.5862 0 0.5] Spawn Lights
  (for (_array_element _array_index) (Variables|Default|GetPlaques)
    (EventDispatchers|BindEventtoHasBeenActivated _array_element (delegate Custom|check))
    (bind _returnvalue_2 (Game|SpawnActorfromClass "/Game/Dev/Bp_Interact/BP_Light.BP_Light_C" (Math|Transform|MakeTransform (+ (+ (* (Transformation|GetActorForwardVector) (Utilities|Select :Index _array_index :Option%200 0.0 :Option%201 1e+02 :Option%202 -1e+02)) (.location _returnvalue)) "0.000000,0.000000,500.000000") (Math|Rotator|MakeRotator 0.0 0.0 (.yaw (.rotation _returnvalue))) "1.000000,1.000000,1.000000") "Undefined" "MultiplyWithRoot" 0 0))
    (Variables|/Game/Dev/Bp_Interact/BP_Light.BP_Light_C|SetPushOn_ref _returnvalue_2 _array_element)
    (Default|GetRef _returnvalue_2))
  (if (Variables|Default|GetBFirstDoor)
    ;[0.01176 0.5781 0 0.5] Check Open
    (Components|Timeline|SetPlayRate (Variables|Default|GetDoor%20Activ) (/ 1.0 (Variables|Default|GetTime%20Opening)))
    (bind _location (Timeline|Door%20Activ Play)
      (:Update
        (Transformation|SetRelativeLocation _sm_door_l_staticmeshcomponent0 (Math|Vector|MakeVector (.x _relativelocation) (.y _relativelocation) (Math|Float|Lerp 0.0 3.9e+02 _location)) false false))
      (:Finished
        (if (Variables|Default|GetBFinalDoor)
          (if (Utilities|IsValidSoftObjectReference _savezone)
            (Variables|/Game/Dev/Checkpoint/BP_SaveZone.BP_SaveZone_C|SetCurrentLevel (Utilities|ResolveSoftReference _savezone) (Variables|Default|GetNextLevel))
            (Variables|/Game/Dev/Checkpoint/BP_SaveZone.BP_SaveZone_C|SetLevelToUnload (Utilities|ResolveSoftReference _savezone) (Variables|Default|GetLevelToUnload))
            (Default|OpenDoors (Variables|/Game/Dev/Checkpoint/BP_SaveZone.BP_SaveZone_C|GetOpeningDoor (Utilities|ResolveSoftReference _savezone)))))))))

(fn ConstructionScript)